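; Third-person character Blueprint that creates the W_Principal UI on BeginPlay and controls its card display from the keyboard.
; Holding key 1, 2 or 3 passes that card's index to MudaImageCard on the widget, and releasing it calls LimpaTela.
; Each press looks the widget up with GetAllWidgetsOfClass instead of keeping the created reference, and the release reuses that result.
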(event EventBeginPlay
  (bind _returnvalue (UserInterface|CreateWidget "/Game/Widgets/W_Principal.W_Principal_C"))
  (UserInterface|Viewport|AddtoViewport _returnvalue 0))

(event Collision|EventActorBeginOverlap
  (params (OtherActor :type Actor%20Object%20Reference)))

(event EventTick
  (params (DeltaSeconds :type Float%20%28single-precision%29)))

(event Input|KeyboardEvents|2
  (params (Key :type Key%20Structure))
  (:Pressed
    (bind _foundwidgets (Widget|GetAllWidgetsOfClass "/Game/Widgets/W_Principal.W_Principal_C" true))
    (Default|MudaImageCard (Utilities|Array|Get(acopy) _foundwidgets) 1))
  (:Released
    (Default|LimpaTela (Utilities|Array|Get(acopy) _foundwidgets))))

(event Input|KeyboardEvents|1
  (params (Key :type Key%20Structure))
  (:Pressed
    (bind _foundwidgets (Widget|GetAllWidgetsOfClass "/Game/Widgets/W_Principal.W_Principal_C" true))
    (Default|MudaImageCard (Utilities|Array|Get(acopy) _foundwidgets)))
  (:Released
    (Default|LimpaTela (Utilities|Array|Get(acopy) _foundwidgets))))

(event Input|KeyboardEvents|3
  (params (Key :type Key%20Structure))
  (:Pressed
    (bind _foundwidgets (Widget|GetAllWidgetsOfClass "/Game/Widgets/W_Principal.W_Principal_C" true))
    (Default|MudaImageCard (Utilities|Array|Get(acopy) _foundwidgets) 2))
  (:Released
    (Default|LimpaTela (Utilities|Array|Get(acopy) _foundwidgets))))

(fn ConstructionScript)